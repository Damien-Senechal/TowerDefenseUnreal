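; BP_Enemy is a tower defense enemy that walks from its spawn to the End actor.
; On BeginPlay, AIMove waits briefly, applies its MaxWalkSpeed to the movement component, then runs AI MoveTo toward the first End actor found.
; A failed move calls AIMove again to retry.
; On arrival the enemy destroys itself and decrements TotalNumberOfEnemies on the TowerDefenseGameMode.
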(event `self.ReceiveBeginPlay`
  (`self.AIMove`))

(event `AIMove`
  (`KismetSystemLibrary.Delay` 0.2)
  (set `CharacterMovementComponent.MaxWalkSpeed` (`self.Max Walk Speed`) (`self.CharacterMovement`))
  (bind _outactors (`GameplayStatics.GetAllActorsOfClass` "/Game/GameObjects/LevelElements/End.End_C"))
  (`|AIMoveTo` self (0.0 0.0 0.0) (`|GetArrayItem` _outactors)
    (:`OnSuccess`
      (`self.K2_DestroyActor`)
      (bind _astower_defense_game_mode (cast `/Game/BP/TowerDefenseGameMode` (`GameplayStatics.GetGameMode`)))
      (bind _output_get (set `self.GameMode` _astower_defense_game_mode))
      (set `/Game/BP/TowerDefenseGameMode.TotalNumberOfEnemies` (- (`/Game/BP/TowerDefenseGameMode.TotalNumberOfEnemies` _output_get) 1) _output_get))
    (:`OnFail`
      (`self.AIMove`))))

(fn `UserConstructionScript`)