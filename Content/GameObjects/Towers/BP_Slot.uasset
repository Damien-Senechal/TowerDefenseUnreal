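; BP_Slot is a clickable tower placement slot that opens the tower selection UI.
; Cursor and click events on its Cube swap materials to show hover, idle, pressed and disabled states.
; When CanSpawnATurret is true, a click removes any existing WB_TowerSelect widgets and creates a new one, passing itself as EmptySlot.
; The slot only reads that flag and contains no spawning logic of its own.
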(event `self.Cube.OnBeginCursorOver`
  (params (TouchedComponent :type "PrimitiveComponent Object Reference"))
  (`PrimitiveComponent.SetMaterial` (`self.Cube`) 0 "/Game/Materials/M_TurretMouseOver.M_TurretMouseOver"))

(event `self.Cube.OnEndCursorOver`
  (params (TouchedComponent :type "PrimitiveComponent Object Reference"))
  (`PrimitiveComponent.SetMaterial` (`self.Cube`) 0 "/Game/Materials/M_TurretMouseOut.M_TurretMouseOut"))

(event `self.Cube.OnClicked`
  (params (TouchedComponent :type "PrimitiveComponent Object Reference") (ButtonPressed :type "Key Structure"))
  (if (`self.CanSpawnATurret`)
    (`PrimitiveComponent.SetMaterial` (`self.Cube`) 0 "/Game/Materials/M_TurretMouseClicked.M_TurretMouseClicked")
    (bind _foundwidgets (`WidgetBlueprintLibrary.GetAllWidgetsOfClass` "/Game/HUD/WB_TowerSelect.WB_TowerSelect_C" false))
    (for _array_element _foundwidgets
      (`Widget.RemoveFromParent` _array_element))
    (bind _returnvalue (`|CreateWidget` "/Game/HUD/WB_TowerSelect.WB_TowerSelect_C"))
    (`UserWidget.AddToViewport` _returnvalue 0)
    (set `/Game/HUD/WB_TowerSelect.EmptySlot` self _returnvalue)
    (else
      (`PrimitiveComponent.SetMaterial` (`self.Cube`) 0 "/Game/Materials/M_TurretMouseDisabled.M_TurretMouseDisabled"))))

(event `self.Cube.OnReleased`
  (params (TouchedComponent :type "PrimitiveComponent Object Reference") (ButtonReleased :type "Key Structure"))
  (`PrimitiveComponent.SetMaterial` (`self.Cube`) 0 "/Game/Materials/M_TurretMouseOver.M_TurretMouseOver"))

(fn `UserConstructionScript`)