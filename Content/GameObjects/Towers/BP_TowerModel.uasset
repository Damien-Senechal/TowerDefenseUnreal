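; Tower actor that detects enemies in range, turns its mesh toward one and fires projectiles from the cannon.
; Overlap events maintain the in-range list, from which a random target is picked and kept until it leaves or its HP check fails.
; Gated, frame-length Delay loops replace Tick, driving constant-speed yaw tracking with delayed shots, or easing the mesh back to zero rotation when no target remains.
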(event `SelectTarget`
  (bind _targetinrange (`self.TargetInRange`))
  (if (`KismetArrayLibrary.Array_IsValidIndex` _targetinrange)
    (set `self.TargetEnemyDetected` (`|GetArrayItem` _targetinrange (`KismetMathLibrary.RandomIntegerInRange` 0 (`KismetArrayLibrary.Array_LastIndex` _targetinrange))))
    (`self.BeginAim`)
    (else
      (`self.ResetAim`))))

(event `self.OverlapDetection.OnComponentBeginOverlap`
  (params (OverlappedComponent :type "PrimitiveComponent Object Reference") (OtherActor :type "Actor Object Reference") (OtherComp :type "PrimitiveComponent Object Reference") (OtherBodyIndex :type Integer) (bFromSweep :type Boolean) (SweepResult :type "HitResult Structure (by ref)"))
  (bind _asbp_enemy (cast `/Game/GameObjects/Enemies/BP_Enemy` OtherActor))
  (`KismetArrayLibrary.Array_Add` (`self.TargetInRange`) _asbp_enemy)
  (`/Engine/EditorBlueprintResources/StandardMacros.IsValid` (`self.TargetEnemyDetected`)
    (:`Is Not Valid`
      (`self.SelectTarget`))))

(event `self.OverlapDetection.OnComponentEndOverlap`
  (params (OverlappedComponent :type "PrimitiveComponent Object Reference") (OtherActor :type "Actor Object Reference") (OtherComp :type "PrimitiveComponent Object Reference") (OtherBodyIndex :type Integer))
  (bind _targetinrange (`self.TargetInRange`))
  (bind _asbp_enemy (cast `/Game/GameObjects/Enemies/BP_Enemy` OtherActor))
  (if (`KismetArrayLibrary.Array_Contains` _targetinrange _asbp_enemy)
    (`KismetArrayLibrary.Array_RemoveItem` _targetinrange _asbp_enemy)
    (if (== (`self.TargetEnemyDetected`) _asbp_enemy)
      (set `self.TargetEnemyDetected` null)
      (`self.SelectTarget`))))

(event `BeginAim`
  (`|ExecutionSequence`
    (:`then_0`
      (goto _label :!via `Open`))
    (:`then_1`
      (`/Engine/EditorBlueprintResources/StandardMacros.Gate` true :!label _label
        (:`Exit`
          (`/Engine/EditorBlueprintResources/StandardMacros.IsValid` (`self.TargetEnemyDetected`)
            (:`Is Valid`
              (`|ExecutionSequence`
                (:`then_0`
                  (`KismetSystemLibrary.Delay` (`self.ShootRate`))
                  (`self.Shoot` self (`self.ProjectileClass`)))
                (:`then_1`
                  (set `self.TargetLocation` (`self.K2_GetActorLocation` (`self.TargetEnemyDetected`)))
                  (`SceneComponent.K2_SetRelativeRotation` (`self.Mesh`) (`KismetMathLibrary.RInterpTo_Constant` (`SceneComponent.RelativeRotation` (`self.Mesh`)) (`KismetMathLibrary.MakeRotator` 0.0 0.0 (+ (.yaw (`KismetMathLibrary.MakeRotFromX` (`KismetMathLibrary.InverseTransformDirection` (`self.GetTransform`) (- (`self.TargetLocation`) (`SceneComponent.K2_GetComponentLocation` (`self.Mesh`)))))) -90.0)) (`GameplayStatics.GetWorldDeltaSeconds`) (`self.RotationSpeed`)) false false)
                  (`KismetSystemLibrary.Delay` (`GameplayStatics.GetWorldDeltaSeconds`))
                  (`self.ContinueAim`))))
            (:`Is Not Valid`
              (`self.CancelAim` :!label _label_2)
              (`self.ResetAim`))))))))

(event `ContinueAim`
  (bind _targetenemydetected (`self.TargetEnemyDetected`))
  (bind _targetinrange (`self.TargetInRange`))
  (bind _targetenemydetected_2 (`self.TargetEnemyDetected`))
  (`/Engine/EditorBlueprintResources/StandardMacros.IsValid` _targetenemydetected
    (:`Is Valid`
      (if (`/Game/GameObjects/Enemies/BP_Enemy.HPGood?` _targetenemydetected)
        (goto _label)
        (elif (`KismetArrayLibrary.Array_Contains` _targetinrange _targetenemydetected_2)
          (`KismetArrayLibrary.Array_RemoveItem` _targetinrange _targetenemydetected_2)
          (set `self.TargetEnemyDetected` null)
          (`self.SelectTarget`))))
    (:`Is Not Valid`
      (goto _label_2))))

(event `CancelAim`
  (goto _label :!via `Close`))

(event `ContinueReset`
  (bind _returnvalue (`KismetMathLibrary.RInterpTo_Constant` (`SceneComponent.RelativeRotation` (`self.Mesh`)) (struct) (`GameplayStatics.GetWorldDeltaSeconds`)))
  (`/Engine/EditorBlueprintResources/StandardMacros.Gate` true :!label _label_3
    (:`Exit`
      (`/Engine/EditorBlueprintResources/StandardMacros.IsValid` (`self.TargetEnemyDetected`)
        (:`Is Valid`
          (`self.StopReset` :!label _label_4))
        (:`Is Not Valid`
          (if (== _returnvalue (struct))
            (goto _label_4)
            (else
              (`SceneComponent.K2_SetRelativeRotation` (`self.Mesh`) _returnvalue false false)
              (`KismetSystemLibrary.Delay` (`GameplayStatics.GetWorldDeltaSeconds`))
              (`self.ContinueReset`))))))))

(event `ResetAim`
  (`|ExecutionSequence`
    (:`then_0`
      (goto _label_3 :!via `Open`))
    (:`then_1`
      (goto _label_3))))

(event `StopReset`
  (goto _label_3 :!via `Close`))

(fn `Shoot`
  (params (ProjectileClass :type "/Game/GameObjects/Towers/Projectiles/BP_Projectiles Class Reference"))
  (`|SpawnActorFromClass` ProjectileClass (`SceneComponent.K2_GetComponentToWorld` (`self.OutCanon`)) "Undefined" "OverrideRootScale" null null)
  (set `self.Projectile` null))

(fn `UserConstructionScript`)