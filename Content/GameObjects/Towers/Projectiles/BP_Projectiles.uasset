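; BP_Projectiles is a tower projectile that damages enemies on impact.
; On BeginPlay it copies its gravity, initial speed and max speed variables into the ProjectileMovement component.
; A SphereHit component hit applies DamageValue to BP_Enemy actors, then plays the hit effect and sound and destroys the projectile whatever it struck.
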(event `self.ReceiveBeginPlay`
  (bind _projectilemovement (`self.ProjectileMovement`))
  (set `ProjectileMovementComponent.ProjectileGravityScale` (`self.ProjectileGravity`) _projectilemovement)
  (set `ProjectileMovementComponent.InitialSpeed` (`self.ProjectileInitialSpeed`) _projectilemovement)
  (set `ProjectileMovementComponent.MaxSpeed` (`self.ProjectileMaxSpeed`) _projectilemovement))

(event `self.ReceiveActorBeginOverlap`
  (params (OtherActor :type "Actor Object Reference")))

(event `self.SphereHit.OnComponentHit`
  (params (HitComponent :type "PrimitiveComponent Object Reference") (OtherActor :type "Actor Object Reference") (OtherComp :type "PrimitiveComponent Object Reference") (NormalImpulse :type "Vector Structure") (Hit :type "HitResult Structure (by ref)"))
  (`|ExecutionSequence`
    (:`then_0`
      (bind _asbp_enemy (cast `/Game/GameObjects/Enemies/BP_Enemy` OtherActor))
      (`GameplayStatics.ApplyDamage` _asbp_enemy (`self.DamageValue`)))
    (:`then_1`
      (`NiagaraFunctionLibrary.SpawnSystemAtLocation` (`self.FxHit`) (`self.K2_GetActorLocation`))
      (`GameplayStatics.SpawnSound2D` (`self.SoundHit`) 1.0 1.0 0.0 null)
      (`self.K2_DestroyActor`))))

(fn `UserConstructionScript`)