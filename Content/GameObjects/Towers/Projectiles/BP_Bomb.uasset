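; Tower bomb projectile that briefly slows any BP_Enemy it overlaps.
; On overlap it runs the inherited parent handler first, then casts the other actor to BP_Enemy and reduces its CharacterMovement max walk speed.
; The prior speed is saved in one variable on the bomb and restored after a short Delay on that same actor, with no per-enemy tracking.
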(event `self.ReceiveActorBeginOverlap`
  (params (OtherActor :type "Actor Object Reference"))
  (`|ExecutionSequence`
    (:`then_0`
      (`parent.ReceiveActorBeginOverlap` OtherActor))
    (:`then_1`
      (bind _asbp_enemy (cast `/Game/GameObjects/Enemies/BP_Enemy` OtherActor))
      (bind _charactermovement (`Character.CharacterMovement` _asbp_enemy))
      (bind _output_get (set `self.InitialMaxWalkSpeed` (`CharacterMovementComponent.MaxWalkSpeed` _charactermovement)))
      (set `CharacterMovementComponent.MaxWalkSpeed` (/ _output_get 1.2) _charactermovement)
      (`KismetSystemLibrary.Delay` 1.0)
      (set `CharacterMovementComponent.MaxWalkSpeed` (`self.InitialMaxWalkSpeed`) _charactermovement))))

(fn `UserConstructionScript`
  (`parent.UserConstructionScript`))